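; Base item object, likely for a grid inventory, that stores its dimensions, rotation state and icon.
; Rotate toggles the Rotated flag and swaps the X and Y dimensions, returning the new size and state.
; GetIcon returns the rotated or normal icon variant to match the current orientation.
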(fn `GetIcon`
  (returns (Icon :type "MaterialInterface Object Reference"))
  (return (select `bool` (`self.Rotated`) :`false` (`self.Icon`) :`true` (`self.IconRotated`))))

(fn `Rotate`
  (returns (NewDimension :type "IntPoint Structure") (IsRotated :type Boolean))
  (bind (_dimensions_x _dimensions_y) (break `IntPoint` (`self.Dimensions`)))
  (if (not (`self.Rotated`))
    (set `self.Rotated` true)
    (else
      (set `self.Rotated` false)))
  (bind _output_get (set `self.Dimensions` (make `IntPoint` _dimensions_y _dimensions_x)))
  (return _output_get (`self.Rotated`)))