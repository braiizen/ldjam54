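; BP_Walker is an enemy that chases the player and destroys itself on contact to deal damage.
; Each Tick, MoveTowardsPlayer pushes the Cylinder toward the Player with a velocity-change impulse scaled by Speed and delta time, so movement is physics-driven and ignores mass.
; When the Sphere overlaps a BP_TopDownChar, it applies fixed damage to that character and calls Die, which is defined outside these graphs.
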(event `self.ReceiveTick`
  (params (DeltaSeconds :type "Float (single-precision)"))
  (`parent.ReceiveTick` DeltaSeconds)
  (`self.MoveTowardsPlayer` DeltaSeconds))

(event `self.Sphere.OnComponentBeginOverlap`
  (params (OverlappedComponent :type "PrimitiveComponent Object Reference") (OtherActor :type "Actor Object Reference") (OtherComp :type "PrimitiveComponent Object Reference") (OtherBodyIndex :type Integer) (bFromSweep :type Boolean) (SweepResult :type "HitResult Structure (by ref)"))
  (bind _asbp_top_down_char (cast `/Game/Character/BP_TopDownChar` OtherActor))
  (`/Game/Character/BP_TopDownChar.TakeDamage` _asbp_top_down_char 20.0)
  (`self.Die`))

(fn `MoveTowardsPlayer`
  (params (Delta :type "Float (double-precision)"))
  (`PrimitiveComponent.AddImpulse` (`self.Cylinder`) (* (`KismetMathLibrary.GetDirectionUnitVector` (`self.K2_GetActorLocation`) (`self.K2_GetActorLocation` (`self.Player`))) (* (`self.Speed`) Delta)) "None" true))

(fn `UserConstructionScript`
  (`parent.UserConstructionScript`))