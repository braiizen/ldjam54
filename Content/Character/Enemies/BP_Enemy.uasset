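; BP_Enemy is an enemy that takes damage, dies and drops loot for the top-down player character.
; AnyDamage shows floating damage numbers and reduces health through HpSystem, which decides when Die runs.
; Die plays a crush sound, drops coin, experience and a possible loot-table item, then destroys the actor.
; The loot table and the spawning of pickups both belong to the player, whose reference is cached on BeginPlay.
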(event `self.ReceiveBeginPlay`
  (`parent.ReceiveBeginPlay`)
  (`/Game/Character/HpSystem.Initialize` (`self.HpSystem`) 0.0)
  (bind _asbp_top_down_char (cast `/Game/Character/BP_TopDownChar` (`GameplayStatics.GetPlayerCharacter` 0)))
  (set `self.Player` _asbp_top_down_char))

(event `self.ReceiveAnyDamage`
  (params (Damage :type "Float (single-precision)") (DamageType :type "DamageType Object Reference") (InstigatedBy :type "Controller Object Reference") (DamageCauser :type "Actor Object Reference"))
  (`self.TakeDamage` Damage))

(fn `Die`
  (`GameplayStatics.PlaySound2D` "/Game/Sounds/Sounds/crush.crush" 1.0 1.0 0.0 null null)
  (`self.DropLoot`)
  (`self.K2_DestroyActor`))

(fn `DropItem`
  (params (Class :type "Actor Class Reference"))
  (bind (_returnvalue_x _returnvalue_y) (`KismetMathLibrary.BreakVector` (`self.K2_GetActorLocation`)))
  (bind _asbp_item_pickup_base (castclass `/Game/Items/BP_ItemPickupBase` Class))
  (`/Game/Character/BP_TopDownChar.SpawnLoot` (`self.Player`) (`KismetMathLibrary.MakeVector` _returnvalue_x _returnvalue_y 100.0) _asbp_item_pickup_base))

(fn `DropLoot`
  (`self.DropItem` (`self.CoinDrop`))
  (`self.DropItem` (`self.ExpDrop`))
  (bind (_loot _isdropped) (`/Game/Inventory/BP_LootTable.GetDrops` (`/Game/Character/BP_TopDownChar.BP_LootTable` (`self.Player`))))
  (if _isdropped
    (`self.DropItem` _loot)))

(fn `SetHP`
  (params (HP :type "Float (double-precision)"))
  (bind _hpsystem (`self.HpSystem`))
  (bind _output_get (set `/Game/Character/HpSystem.MaxHP` HP _hpsystem))
  (set `/Game/Character/HpSystem.CurrentHP` _output_get _hpsystem))

(fn `TakeDamage`
  (params (Damage :type "Float (double-precision)"))
  (`/Game/Inventory/DamageNumbers.MakeFloatingNumbers` (`self.DamageNumbers`) (`self.K2_GetActorLocation`) (`KismetMathLibrary.FTrunc` Damage))
  (bind _isalive (`/Game/Character/HpSystem.ChangeHp` (`self.HpSystem`) (* Damage -1.0)))
  (if (not _isalive)
    (`self.Die`)))

(fn `UserConstructionScript`
  (`parent.UserConstructionScript`))