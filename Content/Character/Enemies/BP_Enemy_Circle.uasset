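; BP_Enemy_Circle is an enemy that periodically fires projectiles through a ProjCall_Enemy_Circle spawner.
; On BeginPlay it spawns that spawner at its root, caches all BP_Object actors and starts a looping timer at the AttackSpeed interval.
; Each tick of the timer moves the spawner's origin to the Cylinder component, then passes loop amount, spawn count and loop speed to the spawner, which handles the actual firing.
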(event `self.ReceiveBeginPlay`
  (`parent.ReceiveBeginPlay`)
  (bind _returnvalue (`|SpawnActorFromClass` "/Game/FX/ProjCall_Enemy_Circle.ProjCall_Enemy_Circle_C" (`KismetMathLibrary.MakeTransform` (`SceneComponent.K2_GetComponentLocation` (`self.DefaultSceneRoot`)) (`KismetMathLibrary.Conv_VectorToRotator` (`KismetMathLibrary.Vector_Zero`))) "Undefined" "MultiplyWithRoot" null (0.0 0.0 0.0) null))
  (set `self.ProjectileSpawner` _returnvalue)
  (bind _outactors (`GameplayStatics.GetAllActorsOfClass` "/Game/Character/Enemies/BP_Object.BP_Object_C"))
  (set `self.Objects` _outactors)
  (bind _returnvalue_2 (`KismetSystemLibrary.K2_SetTimerDelegate` (delegate `E_ShootProjectile`) (`self.AttackSpeed`) true))
  (set `self.ShootTimer` _returnvalue_2))

(event `E_ShootProjectile`
  (`self.ShootProjectile`))

(fn `ShootProjectile`
  (bind _projectilespawner (`self.ProjectileSpawner`))
  (`/Game/FX/ProjCall_Enemy_Circle.Update Origin` _projectilespawner (`SceneComponent.K2_GetComponentLocation` (`self.Cylinder`)))
  (`/Game/FX/ProjCall_Enemy_Circle.ShootProjectile` _projectilespawner (`self.LoopAmount`) (`self.SpawnCount`) (`self.LoopSpeed`)))

(fn `UserConstructionScript`
  (`parent.UserConstructionScript`))